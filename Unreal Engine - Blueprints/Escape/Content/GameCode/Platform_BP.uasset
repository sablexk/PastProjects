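; Moving platform that travels toward an end point while the player is inside its touch trigger and heads back when they leave.
; On BeginPlay it caches the world locations of the platform and the EndPoint component and applies a configurable play rate to the Movement timeline.
; ReadyPlayer overlaps play or reverse that timeline, whose track lerps the platform between both locations without sweeping.
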(event `self.ReceiveBeginPlay`
  (set `self.StartLoc` (`SceneComponent.K2_GetComponentLocation` (`self.Platformer`)))
  (set `self.EndLoc` (`SceneComponent.K2_GetComponentLocation` (`self.End_Point`)))
  (`TimelineComponent.SetPlayRate` (`self.Movement`) (`self.PlayRate`)))

(event `self.Player_Touch.OnComponentBeginOverlap`
  (params (OverlappedComponent :type "PrimitiveComponent Object Reference") (OtherActor :type "Actor Object Reference") (OtherComp :type "PrimitiveComponent Object Reference") (OtherBodyIndex :type Integer) (bFromSweep :type Boolean) (SweepResult :type "HitResult Structure (by ref)"))
  (cast `/Game/GameCode/ReadyPlayer` OtherActor)
  (bind (_direction _newtrack_0) (`Timeline|Movement` :!label _label)
    (:`Update`
      (`SceneComponent.K2_SetWorldLocation` (`self.Platformer`) (`KismetMathLibrary.VLerp` (`self.StartLoc`) (`self.EndLoc`) _newtrack_0) false false))))

(event `self.Player_Touch.OnComponentEndOverlap`
  (params (OverlappedComponent :type "PrimitiveComponent Object Reference") (OtherActor :type "Actor Object Reference") (OtherComp :type "PrimitiveComponent Object Reference") (OtherBodyIndex :type Integer))
  (cast `/Game/GameCode/ReadyPlayer` OtherActor)
  (goto _label :!via `Reverse`))

(fn `UserConstructionScript`)